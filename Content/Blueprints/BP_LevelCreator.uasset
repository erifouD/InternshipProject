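; BP_LevelCreator updates the player's lives and level progress when it ends play.
; On EndPlay it casts the player pawn to BP_PlayerPawn and, if the pawn's InLinePtr is invalid and this element is not a dot, deducts a life and removes a heart.
; It then asks the pawn whether all elements are destroyed and, if so, passes the level.
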(event EventEndPlay
  (params (EndPlayReason :type EEndPlayReason%20Enum :default "Destroyed"))
  (bind _asbp_player_pawn (Utilities|Casting|CastToBP_PlayerPawn (Game|Player|GetPlayerPawn 0)))
  (Utilities|IsValid (Variables|/Script/IntershipSwipeSt.PlayerPawnBase|GetInLinePtr _asbp_player_pawn)
    (:Is%20Valid
      _)
    (:Is%20Not%20Valid
      (if (Class|LevelCreator|BIsElementIsDot)
        _
        (else
          (Math|Integer|DecrementInt (Variables|/Script/IntershipSwipeSt.PlayerPawnBase|GetCurrentLives _asbp_player_pawn)
            (:%20%20
              (Default|HardRemoveHeart _asbp_player_pawn)))))))
  (if (Class|PlayerPawnBase|IsAllElementsDestroyed _asbp_player_pawn)
    (Default|PassLevel _asbp_player_pawn)))

(fn ConstructionScript)