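; BP_Line is an actor that draws a line at runtime by extending a spline with meshes.
; AddSplineElement appends a world-space point from X and Y, makes it linear, then calls SplineMeshCreating.
; That function adds a SplineMeshComponent from the previous point to the new one in local space.
; Each segment reuses the previous point's tangent at both ends.
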(event EventAddSplineElement
  (params (x :type Float%20%28single-precision%29) (y :type Float%20%28single-precision%29))
  (bind _spline (Variables|Default|GetSpline))
  (bind _returnvalue (Spline|GetNumberOfSplinePoints _spline))
  (bind _returnvalue_2 (- _returnvalue 1))
  (Spline|AddSplinePoint (Variables|Default|GetSpline) (Math|Vector|MakeVector x y 0.0) "World" true)
  (Spline|SetSplinePointType _spline _returnvalue_2 "Linear" true)
  (CallFunction|SplineMeshCreating _returnvalue_2))

(fn ConstructionScript)

(fn SplineMeshCreating
  (params (PointIndex :type Integer))
  (bind _returnvalue (- PointIndex 1))
  (bind _spline (Variables|Default|GetSpline))
  (bind (_location _tangent) (Spline|GetLocationandTangentatSplinePoint _spline _returnvalue "Local"))
  (bind _returnvalue_2 (AddComponent|AddSplineMeshComponent false))
  (SplineMesh|SetStartandEnd _returnvalue_2 _location _tangent (Spline|GetLocationatSplinePoint _spline PointIndex "Local") _tangent true :!class /Script/Engine.SplineMeshComponent))